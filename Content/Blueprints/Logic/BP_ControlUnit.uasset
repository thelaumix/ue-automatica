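; BP_ControlUnit is a logic control unit whose construction script builds an optional built-in segment display for its command limit.
; When InternalLimitDisplay is enabled, it spawns the display as a child actor, scaled and positioned from the screen dimensions.
; It sizes the digit count with a base-10 logarithm of CommandLimit and tints the display with the output channel's color.
; Otherwise, it clears the display reference.
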(fn `UserConstructionScript`
  (bind _screenheight (`self.ScreenHeight`))
  (bind _returnvalue (/ _screenheight 60.0))
  (bind _returnvalue_2 (* _returnvalue 0.35))
  (bind _returnvalue_3 (* _returnvalue 5.0))
  (if (`self.Internal Limit Display`)
    (bind _returnvalue_4 (`AddComponent|NODE_AddChildActorComponent-0`))
    (bind _assegment_display (cast `SegmentDisplay` (`ChildActorComponent.ChildActor` _returnvalue_4)))
    (bind _output_get (set `self.LimitDisplay` _assegment_display))
    (`SegmentDisplay.SetNullerDimness` _output_get 0.01)
    (`SceneComponent.K2_SetRelativeTransform` _returnvalue_4 (`KismetMathLibrary.MakeTransform` (`KismetMathLibrary.MakeVector` (- (`self.ScreenWidth`) _returnvalue_3) 0.2 (- (/ _screenheight 2.0) _returnvalue_3)) (struct :`Yaw` 90.0) (`KismetMathLibrary.MakeVector` _returnvalue_2 _returnvalue_2 _returnvalue_2)) false false)
    (`SegmentDisplay.SetDigits` _output_get (+ (`KismetMathLibrary.Conv_IntToByte` (`KismetMathLibrary.FFloor` (`KismetMathLibrary.Log` (`KismetMathLibrary.Conv_ByteToDouble` (`self.CommandLimit`)) 10.0))) 1))
    (bind _returnvalue_5 (`Automatica.GetChannelColor` (`self.ChannelOut`)))
    (`SegmentDisplay.SetColor` _output_get _returnvalue_5)
    (else
      (set `self.LimitDisplay` null))))