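; Player pawn that configures itself for VR or desktop at BeginPlay, depending on whether a head-mounted display is enabled.
; VR attaches InteractionCatchers to both hands; desktop hides the hands and moves one catcher along a short view trace each Tick.
; Click or shoot inputs press the button the relevant catcher has caught.
; Enhanced Input also drives movement, clamped mouse look and hand pose alphas in ABP_MannequinsXR.
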(event `self.ReceiveBeginPlay`
  (bind _returnvalue (pcsubsystem `EnhancedInputLocalPlayerSubsystem` (`GameplayStatics.GetPlayerController` 0)))
  (bind _output_get (set `self.VR Mode` (`HeadMountedDisplayFunctionLibrary.IsHeadMountedDisplayEnabled`)))
  (if _output_get
    (bind _returnvalue_2 (`AddComponent|NODE_AddInteractionCatcher-1` :`bManualAttachment` true))
    (`SceneComponent.K2_AttachToComponent` _returnvalue_2 (`self.HandLeft`) "None" "SnapToTarget" "SnapToTarget" "SnapToTarget" true)
    (bind _output_get_2 (set `self.Catcher_LH` _returnvalue_2))
    (`SceneComponent.K2_SetRelativeLocation` _output_get_2 (`SceneComponent.RelativeLocation` (`self.GAnchorLeft`)) false false)
    (bind _returnvalue_3 (`AddComponent|NODE_AddInteractionCatcher-2` :`bManualAttachment` true))
    (`SceneComponent.K2_AttachToComponent` _returnvalue_3 (`self.HandRight`) "None" "SnapToTarget" "SnapToTarget" "SnapToTarget" true)
    (bind _output_get_3 (set `self.Catcher_RH` _returnvalue_3))
    (`SceneComponent.K2_SetRelativeLocation` _output_get_3 (`SceneComponent.RelativeLocation` (`self.GAnchorRight`)) false false)
    (`HeadMountedDisplayFunctionLibrary.SetWorldToMetersScale` 100.0)
    (`HeadMountedDisplayFunctionLibrary.SetTrackingOrigin` "Eye")
    (`KismetSystemLibrary.ExecuteConsoleCommand` "vr.PixelDensity 1.0" null)
    (`CapsuleComponent.SetCapsuleHalfHeight` (`self.CapsuleComponent`) 125.0 true)
    (`EnhancedInputSubsystemInterface.AddMappingContext` _returnvalue "/Game/VRTemplate/Input/IMC_Default.IMC_Default" 0 (struct))
    (`EnhancedInputSubsystemInterface.AddMappingContext` _returnvalue "/Game/VRTemplate/Input/IMC_Hands.IMC_Hands" 0 (struct))
    (else
      (bind _returnvalue_4 (`AddComponent|NODE_AddInteractionCatcher-3`))
      (set `self.DesktopCatcher` _returnvalue_4)
      (`CapsuleComponent.SetCapsuleHalfHeight` (`self.CapsuleComponent`) 88.0 true)
      (`SceneComponent.SetHiddenInGame` (`self.HandRight`) true false)
      (`SceneComponent.SetHiddenInGame` (`self.HandLeft`) true false)
      (`EnhancedInputSubsystemInterface.AddMappingContext` _returnvalue "/Game/Blueprints/Input/CTX_Keyboard.CTX_Keyboard" 0 (struct)))))

(event `EnhancedInput|/Game/Blueprints/Input/Actions/IA_Move`
  (params (ActionValue :type "Vector2D Structure") (ElapsedSeconds :type "Float (double-precision)") (TriggeredSeconds :type "Float (double-precision)") (InputAction :type "InputAction Object Reference" :default "/Game/Blueprints/Input/Actions/IA_Move.IA_Move"))
  (bind (_x _y) (`KismetMathLibrary.BreakVector2D` ActionValue))
  (bind _eyes (`self.Eyes`))
  (:`Triggered`
    (`PawnMovementComponent.AddInputVector` (`self.CharacterMovement`) (+ (* _x (`SceneComponent.GetRightVector` _eyes)) (* _y (`KismetMathLibrary.Normal` (`KismetMathLibrary.MakeVector` (.x (`SceneComponent.GetForwardVector` _eyes)) (.y (`SceneComponent.GetForwardVector` _eyes)))))) false)))

(event `EnhancedInput|/Game/Blueprints/Input/Actions/IA_Look`
  (params (ActionValue :type "Vector2D Structure") (ElapsedSeconds :type "Float (double-precision)") (TriggeredSeconds :type "Float (double-precision)") (InputAction :type "InputAction Object Reference" :default "/Game/Blueprints/Input/Actions/IA_Look.IA_Look"))
  (bind (_x _y) (`KismetMathLibrary.BreakVector2D` (* (* ActionValue (`self.MouseSensitivity`)) 2.0)))
  (:`Triggered`
    (`SceneComponent.K2_SetRelativeRotation` (`self.Eyes`) (`KismetMathLibrary.MakeRotator` 0.0 (`KismetMathLibrary.FClamp` (+ (.pitch (`SceneComponent.RelativeRotation` (`self.Eyes`))) _y) -85.0 85.0) (+ (.yaw (`SceneComponent.RelativeRotation` (`self.Eyes`))) _x)) false false)))

(event `EnhancedInput|/Game/VRTemplate/Input/Actions/Hands/IA_Hand_Grasp_Left`
  (params (ActionValue :type "Float (double-precision)") (ElapsedSeconds :type "Float (double-precision)") (TriggeredSeconds :type "Float (double-precision)") (InputAction :type "InputAction Object Reference" :default "/Game/VRTemplate/Input/Actions/Hands/IA_Hand_Grasp_Left.IA_Hand_Grasp_Left"))
  (bind _returnvalue (`SkeletalMeshComponent.GetAnimInstance` (`self.HandLeft`)))
  (:`Triggered`
    (bind _asabp_mannequins_xr (cast `/Game/Characters/MannequinsXR/Meshes/ABP_MannequinsXR` _returnvalue))
    (set `/Game/Characters/MannequinsXR/Meshes/ABP_MannequinsXR.PoseAlphaGrasp` ActionValue _asabp_mannequins_xr))
  (:`Canceled`
    (bind _asabp_mannequins_xr_2 (cast `/Game/Characters/MannequinsXR/Meshes/ABP_MannequinsXR` _returnvalue :!label _label))
    (set `/Game/Characters/MannequinsXR/Meshes/ABP_MannequinsXR.PoseAlphaGrasp` 0.0 _asabp_mannequins_xr_2))
  (:`Completed`
    (goto _label)))

(event `EnhancedInput|/Game/VRTemplate/Input/Actions/Hands/IA_Hand_Grasp_Right`
  (params (ActionValue :type "Float (double-precision)") (ElapsedSeconds :type "Float (double-precision)") (TriggeredSeconds :type "Float (double-precision)") (InputAction :type "InputAction Object Reference" :default "/Game/VRTemplate/Input/Actions/Hands/IA_Hand_Grasp_Right.IA_Hand_Grasp_Right"))
  (bind _returnvalue (`SkeletalMeshComponent.GetAnimInstance` (`self.HandRight`)))
  (:`Triggered`
    (bind _asabp_mannequins_xr (cast `/Game/Characters/MannequinsXR/Meshes/ABP_MannequinsXR` _returnvalue))
    (set `/Game/Characters/MannequinsXR/Meshes/ABP_MannequinsXR.PoseAlphaGrasp` ActionValue _asabp_mannequins_xr))
  (:`Canceled`
    (bind _asabp_mannequins_xr_2 (cast `/Game/Characters/MannequinsXR/Meshes/ABP_MannequinsXR` _returnvalue :!label _label_2))
    (set `/Game/Characters/MannequinsXR/Meshes/ABP_MannequinsXR.PoseAlphaGrasp` 0.0 _asabp_mannequins_xr_2))
  (:`Completed`
    (goto _label_2)))

(event `EnhancedInput|/Game/VRTemplate/Input/Actions/Hands/IA_Hand_IndexCurl_Left`
  (params (ActionValue :type "Float (double-precision)") (ElapsedSeconds :type "Float (double-precision)") (TriggeredSeconds :type "Float (double-precision)") (InputAction :type "InputAction Object Reference" :default "/Game/VRTemplate/Input/Actions/Hands/IA_Hand_IndexCurl_Left.IA_Hand_IndexCurl_Left"))
  (bind _returnvalue (`SkeletalMeshComponent.GetAnimInstance` (`self.HandLeft`)))
  (:`Triggered`
    (bind _asabp_mannequins_xr (cast `/Game/Characters/MannequinsXR/Meshes/ABP_MannequinsXR` _returnvalue))
    (set `/Game/Characters/MannequinsXR/Meshes/ABP_MannequinsXR.PoseAlphaIndexCurl` ActionValue _asabp_mannequins_xr))
  (:`Canceled`
    (bind _asabp_mannequins_xr_2 (cast `/Game/Characters/MannequinsXR/Meshes/ABP_MannequinsXR` _returnvalue :!label _label_3))
    (set `/Game/Characters/MannequinsXR/Meshes/ABP_MannequinsXR.PoseAlphaIndexCurl` 0.0 _asabp_mannequins_xr_2))
  (:`Completed`
    (goto _label_3)))

(event `EnhancedInput|/Game/VRTemplate/Input/Actions/Hands/IA_Hand_IndexCurl_Right`
  (params (ActionValue :type "Float (double-precision)") (ElapsedSeconds :type "Float (double-precision)") (TriggeredSeconds :type "Float (double-precision)") (InputAction :type "InputAction Object Reference" :default "/Game/VRTemplate/Input/Actions/Hands/IA_Hand_IndexCurl_Right.IA_Hand_IndexCurl_Right"))
  (bind _returnvalue (`SkeletalMeshComponent.GetAnimInstance` (`self.HandRight`)))
  (:`Triggered`
    (bind _asabp_mannequins_xr (cast `/Game/Characters/MannequinsXR/Meshes/ABP_MannequinsXR` _returnvalue))
    (set `/Game/Characters/MannequinsXR/Meshes/ABP_MannequinsXR.PoseAlphaIndexCurl` ActionValue _asabp_mannequins_xr))
  (:`Canceled`
    (bind _asabp_mannequins_xr_2 (cast `/Game/Characters/MannequinsXR/Meshes/ABP_MannequinsXR` _returnvalue :!label _label_4))
    (set `/Game/Characters/MannequinsXR/Meshes/ABP_MannequinsXR.PoseAlphaIndexCurl` 0.0 _asabp_mannequins_xr_2))
  (:`Completed`
    (goto _label_4)))

(event `EnhancedInput|/Game/VRTemplate/Input/Actions/Hands/IA_Hand_Point_Left`
  (params (ActionValue :type "Float (double-precision)") (ElapsedSeconds :type "Float (double-precision)") (TriggeredSeconds :type "Float (double-precision)") (InputAction :type "InputAction Object Reference" :default "/Game/VRTemplate/Input/Actions/Hands/IA_Hand_Point_Left.IA_Hand_Point_Left"))
  (bind _handleft (`self.HandLeft`))
  (:`Started`
    (bind _asabp_mannequins_xr (cast `/Game/Characters/MannequinsXR/Meshes/ABP_MannequinsXR` (`SkeletalMeshComponent.GetAnimInstance` _handleft) :!label _label_5))
    (set `/Game/Characters/MannequinsXR/Meshes/ABP_MannequinsXR.PoseAlphaPoint` 0.0 _asabp_mannequins_xr))
  (:`Canceled`
    (goto _label_5))
  (:`Completed`
    (bind _asabp_mannequins_xr_2 (cast `/Game/Characters/MannequinsXR/Meshes/ABP_MannequinsXR` (`SkeletalMeshComponent.GetAnimInstance` _handleft)))
    (set `/Game/Characters/MannequinsXR/Meshes/ABP_MannequinsXR.PoseAlphaPoint` 1.0 _asabp_mannequins_xr_2)))

(event `EnhancedInput|/Game/VRTemplate/Input/Actions/Hands/IA_Hand_Point_Right`
  (params (ActionValue :type "Float (double-precision)") (ElapsedSeconds :type "Float (double-precision)") (TriggeredSeconds :type "Float (double-precision)") (InputAction :type "InputAction Object Reference" :default "/Game/VRTemplate/Input/Actions/Hands/IA_Hand_Point_Right.IA_Hand_Point_Right"))
  (bind _handright (`self.HandRight`))
  (:`Started`
    (bind _asabp_mannequins_xr (cast `/Game/Characters/MannequinsXR/Meshes/ABP_MannequinsXR` (`SkeletalMeshComponent.GetAnimInstance` _handright) :!label _label_6))
    (set `/Game/Characters/MannequinsXR/Meshes/ABP_MannequinsXR.PoseAlphaPoint` 0.0 _asabp_mannequins_xr))
  (:`Canceled`
    (goto _label_6))
  (:`Completed`
    (bind _asabp_mannequins_xr_2 (cast `/Game/Characters/MannequinsXR/Meshes/ABP_MannequinsXR` (`SkeletalMeshComponent.GetAnimInstance` _handright)))
    (set `/Game/Characters/MannequinsXR/Meshes/ABP_MannequinsXR.PoseAlphaPoint` 1.0 _asabp_mannequins_xr_2)))

(event `EnhancedInput|/Game/VRTemplate/Input/Actions/Hands/IA_Hand_ThumbUp_Left`
  (params (ActionValue :type "Float (double-precision)") (ElapsedSeconds :type "Float (double-precision)") (TriggeredSeconds :type "Float (double-precision)") (InputAction :type "InputAction Object Reference" :default "/Game/VRTemplate/Input/Actions/Hands/IA_Hand_ThumbUp_Left.IA_Hand_ThumbUp_Left"))
  (bind _handleft (`self.HandLeft`))
  (:`Started`
    (bind _asabp_mannequins_xr (cast `/Game/Characters/MannequinsXR/Meshes/ABP_MannequinsXR` (`SkeletalMeshComponent.GetAnimInstance` _handleft) :!label _label_7))
    (set `/Game/Characters/MannequinsXR/Meshes/ABP_MannequinsXR.PoseAlphaThumbUp` 0.0 _asabp_mannequins_xr))
  (:`Canceled`
    (goto _label_7))
  (:`Completed`
    (bind _asabp_mannequins_xr_2 (cast `/Game/Characters/MannequinsXR/Meshes/ABP_MannequinsXR` (`SkeletalMeshComponent.GetAnimInstance` _handleft)))
    (set `/Game/Characters/MannequinsXR/Meshes/ABP_MannequinsXR.PoseAlphaThumbUp` 1.0 _asabp_mannequins_xr_2)))

(event `EnhancedInput|/Game/VRTemplate/Input/Actions/Hands/IA_Hand_ThumbUp_Right`
  (params (ActionValue :type "Float (double-precision)") (ElapsedSeconds :type "Float (double-precision)") (TriggeredSeconds :type "Float (double-precision)") (InputAction :type "InputAction Object Reference" :default "/Game/VRTemplate/Input/Actions/Hands/IA_Hand_ThumbUp_Right.IA_Hand_ThumbUp_Right"))
  (bind _handright (`self.HandRight`))
  (:`Started`
    (bind _asabp_mannequins_xr (cast `/Game/Characters/MannequinsXR/Meshes/ABP_MannequinsXR` (`SkeletalMeshComponent.GetAnimInstance` _handright) :!label _label_8))
    (set `/Game/Characters/MannequinsXR/Meshes/ABP_MannequinsXR.PoseAlphaThumbUp` 0.0 _asabp_mannequins_xr))
  (:`Canceled`
    (goto _label_8))
  (:`Completed`
    (bind _asabp_mannequins_xr_2 (cast `/Game/Characters/MannequinsXR/Meshes/ABP_MannequinsXR` (`SkeletalMeshComponent.GetAnimInstance` _handright)))
    (set `/Game/Characters/MannequinsXR/Meshes/ABP_MannequinsXR.PoseAlphaThumbUp` 1.0 _asabp_mannequins_xr_2)))

(event `self.ReceiveTick`
  (params (DeltaSeconds :type "Float (single-precision)"))
  (bind _eyes (`self.Eyes`))
  (bind _returnvalue (`SceneComponent.K2_GetComponentLocation` _eyes))
  (if (and (not (`self.VR Mode`)) (`KismetSystemLibrary.IsValid` (`self.DesktopCatcher`)))
    (bind _outhit (`KismetSystemLibrary.LineTraceSingle` _returnvalue (+ _returnvalue (* (`SceneComponent.GetForwardVector` _eyes) 220.0)) "TraceTypeQuery2"))
    (`SceneComponent.K2_SetWorldLocation` (`self.DesktopCatcher`) (`.Location` (`GameplayStatics.BreakHitResult` _outhit)) false false)))

(event `EnhancedInput|/Game/Blueprints/Input/Actions/IA_Click`
  (params (ActionValue :type Boolean) (ElapsedSeconds :type "Float (double-precision)") (TriggeredSeconds :type "Float (double-precision)") (InputAction :type "InputAction Object Reference" :default "/Game/Blueprints/Input/Actions/IA_Click.IA_Click"))
  (bind _desktopcatcher (`self.DesktopCatcher`))
  (:`Started`
    (if (and (not (`self.VR Mode`)) (`KismetSystemLibrary.IsValid` _desktopcatcher))
      (`InteractionCatcher.TriggerPressOnCatchedButton` _desktopcatcher))))

(event `EnhancedInput|/Game/VRTemplate/Input/Actions/IA_Shoot_Left`
  (params (ActionValue :type Boolean) (ElapsedSeconds :type "Float (double-precision)") (TriggeredSeconds :type "Float (double-precision)") (InputAction :type "InputAction Object Reference" :default "/Game/VRTemplate/Input/Actions/IA_Shoot_Left.IA_Shoot_Left"))
  (bind _catcher_lh (`self.Catcher_LH`))
  (:`Started`
    (if (and (`KismetSystemLibrary.IsValid` _catcher_lh) (`self.VR Mode`))
      (`InteractionCatcher.TriggerPressOnCatchedButton` _catcher_lh))))

(event `EnhancedInput|/Game/VRTemplate/Input/Actions/IA_Shoot_Right`
  (params (ActionValue :type Boolean) (ElapsedSeconds :type "Float (double-precision)") (TriggeredSeconds :type "Float (double-precision)") (InputAction :type "InputAction Object Reference" :default "/Game/VRTemplate/Input/Actions/IA_Shoot_Right.IA_Shoot_Right"))
  (bind _catcher_rh (`self.Catcher_RH`))
  (:`Started`
    (if (and (`self.VR Mode`) (`KismetSystemLibrary.IsValid` _catcher_rh))
      (`InteractionCatcher.TriggerPressOnCatchedButton` _catcher_rh))))

(fn `UserConstructionScript`)